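; Coin minigame manager that gives players a time limit to get a coin and has those without one killed.
; Activar updates every ThirdPersonCharacter's instruction text and starts two timers.
; One spawns a coin pickup per character at random positions within a square around the world origin.
; The other ends the round, hiding coin display, calling MandarMatar on coinless characters and reporting to GameManagerActor.
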(event `/Game/Blueprints/Interfaces/IActivable.Activar`
  (params (Tiempo :type "Float (single-precision)"))
  ;[0.9447 0.1894 1] Inicializo
  (bind _output_get (set `self.Tiempo De Vida Restante` Tiempo))
  (bind _returnvalue (`GameplayStatics.GetActorOfClass` "/Game/Blueprints/GameManager/GameManagerActor.GameManagerActor_C"))
  (set `self.Referencia a GM` _returnvalue)
  (`self.changeText`)
  (`KismetSystemLibrary.K2_SetTimer` null "destroyMyself" _output_get)
  (`KismetSystemLibrary.K2_SetTimerDelegate` (delegate `hazMonedas`) 1.0 false 0.5))

(event `hazMonedas`
  ;[0.5021 0.869 1] hacerMonedas
  (bind _outactors (`GameplayStatics.GetAllActorsOfClass` "/Game/ThirdPersonBP/Blueprints/ThirdPersonCharacter.ThirdPersonCharacter_C"))
  (for _ _outactors
    (`self.SpawnearMonedas`)))

(event `SpawnearMonedas`
  ;[1 0.2889 0.03704] SpawnMoneditas
  (`|SpawnActorFromClass` "/Game/Blueprints/ObjMonedeable.ObjMonedeable_C" (`KismetMathLibrary.MakeTransform` (`KismetMathLibrary.MakeVector` (`KismetMathLibrary.RandomFloatInRange` -1000.0 1000.0) (`KismetMathLibrary.RandomFloatInRange` -1000.0 1000.0) 200.0)) "Undefined" "OverrideRootScale" null null))

(event `changeText`
  ;[0.7057 1 0.6784] cambiarTexto
  (bind _outactors (`GameplayStatics.GetAllActorsOfClass` "/Game/ThirdPersonBP/Blueprints/ThirdPersonCharacter.ThirdPersonCharacter_C"))
  (for _array_element _outactors
    (`/Game/ThirdPersonBP/Blueprints/ThirdPersonCharacter.cahngeIndication` _array_element "ConsigueUnaMoneda")))

(event `/Game/Blueprints/Interfaces/IReseteable.Resetear`
  ;[1 0.3528 0.9657] Reseteo
  (`self.K2_DestroyActor`))

(fn `destroyMyself`
  (`KismetSystemLibrary.PrintString` "destuirme" true true (struct :`R` 1.0 :`G` 0.144818 :`B` 0.184622 :`A` 1.0) 4.0)
  (bind _outactors (`GameplayStatics.GetAllActorsOfClass` "/Game/ThirdPersonBP/Blueprints/ThirdPersonCharacter.ThirdPersonCharacter_C"))
  (for _array_element _outactors
    (`/Game/ThirdPersonBP/Blueprints/ThirdPersonCharacter.StopShowingMoneditas` _array_element)
    (bind _tiene (`/Game/ThirdPersonBP/Blueprints/ThirdPersonCharacter.askMoneda` _array_element))
    (if (not _tiene)
      (`/Game/ThirdPersonBP/Blueprints/ThirdPersonCharacter.MandarMatar` _array_element)))
  (`/Game/Blueprints/GameManager/GameManagerActor.EndMiniGame` (`self.Referencia a GM`) self))

(fn `Test`)

(fn `UserConstructionScript`)