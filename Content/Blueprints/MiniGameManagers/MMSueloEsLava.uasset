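; Manager actor for the "Suelo Es Lava" (floor is lava) minigame, timing the round and reporting its end.
; BeginPlay calls Activar(0) on the Lava actor and every PlataformaSueloEsLava, while its own Activar only arms a countdown run on Tick.
; On expiry it calls Activar(0) on the lava, then on the platforms after a fixed delay.
; After DelayPostMiniGame it calls EndMiniGame on GameManagerActor.
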(event `self.ReceiveBeginPlay`
  ;[0.717 0.154 1] Condiciones iniciales
  (bind _returnvalue (`GameplayStatics.GetActorOfClass` "/Game/Blueprints/Lava.Lava_C"))
  (`/Game/Blueprints/Interfaces/IActibable.Activar` _returnvalue 0.0)
  (bind _outactors (`GameplayStatics.GetAllActorsOfClass` "/Game/Blueprints/PlataformaSueloEsLava.PlataformaSueloEsLava_C"))
  (for _array_element _outactors
    (`/Game/Blueprints/Interfaces/IActibable.Activar` _array_element 0.0)))

(event `/Game/Blueprints/Interfaces/IActibable.Activar`
  (params (Tiempo :type "Float (single-precision)"))
  ;[0.2573 0.1697 1] Activar
  (set `self.TiempoDeVidaRestante` Tiempo)
  (set `self.Activo` true))

(event `self.ReceiveTick`
  (params (DeltaSeconds :type "Float (single-precision)"))
  ;[0.5294 0.9602 1] Verifica si acabó su tiempo de vida
  (bind _output_get (set `self.TiempoDeVidaRestante` (- (`self.TiempoDeVidaRestante`) DeltaSeconds)))
  (if (and (<= _output_get 0.0) (`self.Activo`))
    ;[1 0.2705 0.7965] Le indica al GameManagerActor que ya acabó
    (set `self.Activo` false)
    (bind _returnvalue (`GameplayStatics.GetActorOfClass` "/Game/Blueprints/Lava.Lava_C"))
    (`/Game/Blueprints/Interfaces/IActibable.Activar` _returnvalue 0.0)
    (`KismetSystemLibrary.Delay` 11.0)
    (bind _outactors (`GameplayStatics.GetAllActorsOfClass` "/Game/Blueprints/PlataformaSueloEsLava.PlataformaSueloEsLava_C"))
    (for _array_element _outactors
      (`/Game/Blueprints/Interfaces/IActibable.Activar` _array_element 0.0))
    (`KismetSystemLibrary.Delay` (`self.DelayPostMiniGame`))
    (bind _returnvalue_2 (`GameplayStatics.GetActorOfClass` "/Game/Blueprints/GameManager/GameManagerActor.GameManagerActor_C"))
    (`/Game/Blueprints/GameManager/GameManagerActor.EndMiniGame` _returnvalue_2 self)))

(fn `UserConstructionScript`)