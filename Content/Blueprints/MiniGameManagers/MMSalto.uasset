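; Mini-game manager for a jump challenge ("Salto") that kills characters who fail to jump before time runs out.
; Activar caches the GameManagerActor, clears HasJumped on every ThirdPersonCharacter and starts a timer for the given duration.
; On expiry, destroyMyself calls MandarMatar on each character whose AskJump returns false, then reports to the game manager through EndMiniGame.
; Actual actor destruction happens in Resetear.
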(event `/Game/Blueprints/Interfaces/IActivable.Activar`
  (params (Tiempo :type "Float (single-precision)"))
  ;[0.9447 0.1894 1] Inicializo
  (bind _output_get (set `self.Tiempo De Vida Restante` Tiempo))
  (bind _returnvalue (`GameplayStatics.GetActorOfClass` "/Game/Blueprints/GameManager/GameManagerActor.GameManagerActor_C"))
  (set `self.Referencia a GM` _returnvalue)
  (`KismetSystemLibrary.PrintString` (`KismetStringLibrary.Conv_DoubleToString` _output_get) true true (struct :`G` 1.0 :`B` 0.152043 :`A` 1.0))
  (`KismetSystemLibrary.K2_SetTimer` null "destroyMyself" _output_get false _output_get)
  (bind _outactors (`GameplayStatics.GetAllActorsOfClass` "/Game/ThirdPersonBP/Blueprints/ThirdPersonCharacter.ThirdPersonCharacter_C"))
  (for _array_element _outactors
    (set `/Game/ThirdPersonBP/Blueprints/ThirdPersonCharacter.hasJumped` false _array_element)))

(event `/Game/Blueprints/Interfaces/IReseteable.Resetear`
  ;[0.5595 0.4855 1] Reseteo
  (`self.K2_DestroyActor`))

(fn `destroyMyself`
  (`KismetSystemLibrary.PrintString` "destuirme" true true (struct :`R` 1.0 :`G` 0.144818 :`B` 0.184622 :`A` 1.0) 4.0)
  (bind _outactors (`GameplayStatics.GetAllActorsOfClass` "/Game/ThirdPersonBP/Blueprints/ThirdPersonCharacter.ThirdPersonCharacter_C"))
  (for _array_element _outactors
    (bind _hasjumped (`/Game/ThirdPersonBP/Blueprints/ThirdPersonCharacter.askJump` _array_element))
    (if (not _hasjumped)
      (`/Game/ThirdPersonBP/Blueprints/ThirdPersonCharacter.MandarMatar` _array_element)))
  (`/Game/Blueprints/GameManager/GameManagerActor.EndMiniGame` (`self.Referencia a GM`) self))

(fn `Test`)

(fn `UserConstructionScript`)