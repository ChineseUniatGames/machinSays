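; Minigame manager that periodically spawns side-to-side objects for a limited lifetime.
; A looping timer spawns each ObjetoLadoALado at GameManagerActor's LimiteX minus Offset, facing its target at LimiteX plus Offset.
; Y always equals LimiteY, as both random-range bounds match.
; Activar sets the lifetime, which Tick counts down, calling EndMiniGame on GameManagerActor every frame it is at or below zero.
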(event `self.ReceiveBeginPlay`
  ;[0.717 0.154 1] Condiciones iniciales
  (`KismetSystemLibrary.PrintString` "Estoy vivo")
  (set `self.TiempoDeVidaRestante` 100.0)
  (bind _returnvalue (`GameplayStatics.GetActorOfClass` "/Game/Blueprints/GameManager/GameManagerActor.GameManagerActor_C"))
  (set `self.ReferenciaLimites` _returnvalue)
  (`KismetSystemLibrary.K2_SetTimer` null "Spawnear YMover" (`self.SpawnRate`) true))

(event `/Game/Blueprints/Interfaces/IActibable.Activar`
  (params (Tiempo :type "Float (single-precision)"))
  ;[0.2573 0.1697 1] Activar
  (set `self.TiempoDeVidaRestante` Tiempo))

(event `self.ReceiveTick`
  (params (DeltaSeconds :type "Float (single-precision)"))
  ;[0.5294 0.9602 1] Verifica si acabó su tiempo de vida
  (bind _output_get (set `self.TiempoDeVidaRestante` (- (`self.TiempoDeVidaRestante`) DeltaSeconds)))
  (if (<= _output_get 0.0)
    ;[1 0.2705 0.7965] Le indica al GameManagerActor que ya acabó
    (bind _returnvalue (`GameplayStatics.GetActorOfClass` "/Game/Blueprints/GameManager/GameManagerActor.GameManagerActor_C"))
    (`/Game/Blueprints/GameManager/GameManagerActor.EndMiniGame` _returnvalue self)))

(fn `Spawnear YMover`
  (bind _referencialimites (`self.ReferenciaLimites`))
  (bind _offset (`/Game/Blueprints/GameManager/GameManagerActor.Offset` _referencialimites))
  (bind _output_get (set `self.VectorTemporal` (`KismetMathLibrary.MakeVector` (- (`/Game/Blueprints/GameManager/GameManagerActor.Limite-X` _referencialimites) _offset) (`KismetMathLibrary.RandomFloatInRange` (`/Game/Blueprints/GameManager/GameManagerActor.Limite-Y` _referencialimites) (`/Game/Blueprints/GameManager/GameManagerActor.Limite+Y` _referencialimites)))))
  (bind _returnvalue (`|SpawnActorFromClass` "/Game/Blueprints/ObjetoLadoALado.ObjetoLadoALado_C" (`KismetMathLibrary.MakeTransform` _output_get (struct)) "Undefined" "OverrideRootScale" null null))
  (bind _returnvalue_2 (`KismetMathLibrary.MakeVector` (+ (`/Game/Blueprints/GameManager/GameManagerActor.Limite+X` _referencialimites) _offset) (.y _output_get) (.z _output_get)))
  (set `/Game/Blueprints/ObjetoLadoALado.Objetivo` _returnvalue_2 _returnvalue)
  (`self.K2_SetActorRotation` _returnvalue (`KismetMathLibrary.FindLookAtRotation` _output_get _returnvalue_2) false))

(fn `UserConstructionScript`)