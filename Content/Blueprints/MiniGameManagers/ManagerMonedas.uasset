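; Coin manager for a minigame that drops ObjMonedeable actors from a fixed height at random horizontal positions.
; BeginPlay waits briefly, then calls RunOnServer through Test.
; RunOnServer sets a looping timer on SpawnearMonedas, which spawns one coin per call.
; Its exec wire loops back from the timer setup to an unused character lookup, forming a cycle with no exit.
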(event `RunOnServer`
  ;[1 0.9436 0.03794] correrEnServer
  (bind _outactors (`GameplayStatics.GetAllActorsOfClass` "/Game/ThirdPersonBP/Blueprints/ThirdPersonCharacter.ThirdPersonCharacter_C" :!label _label))
  (`KismetSystemLibrary.K2_SetTimerDelegate` (delegate `SpawnearMonedas`) 2.0 true)
  (goto _label))

(event `SpawnearMonedas`
  (bind _returnvalue (`KismetMathLibrary.RandomFloatInRange` -1100.0 1100.0))
  ;[1 0.2889 0.03704] SpawnMoneditas
  (`|SpawnActorFromClass` "/Game/Blueprints/ObjMonedeable.ObjMonedeable_C" (`KismetMathLibrary.MakeTransform` (`KismetMathLibrary.MakeVector` _returnvalue _returnvalue 3000.0)) "Undefined" "OverrideRootScale" null null))

(event `self.ReceiveBeginPlay`
  (`KismetSystemLibrary.K2_SetTimer` null "Test" 3.0))

(fn `Test`
  (`self.RunOnServer`))

(fn `UserConstructionScript`)