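; MMCaenDelCielo is a timed minigame actor, judging by its EndMiniGame call, and holds only countdown logic.
; BeginPlay sets a default lifetime, which the Activar event overrides with a given time.
; Tick decrements it and, once expired, calls EndMiniGame on GameManagerActor via GetActorOfClass, repeating every frame without a guard.
; Disconnected nodes retain an unused GameState-based GameManager variant for reading time and ending the minigame.
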(event `self.ReceiveBeginPlay`
  ;[0.717 0.154 1] Condiciones iniciales
  (`KismetSystemLibrary.PrintString` "Estoy vivo")
  (set `self.TiempoDeVidaRestante` 100.0))

(event `/Game/Blueprints/Interfaces/IActibable.Activar`
  (params (Tiempo :type "Float (single-precision)"))
  ;[0.2573 0.1697 1] Activar
  (set `self.TiempoDeVidaRestante` Tiempo))

(event `self.ReceiveTick`
  (params (DeltaSeconds :type "Float (single-precision)"))
  ;[0.5294 0.9602 1] Verifica si acabó su tiempo de vida
  (bind _output_get (set `self.TiempoDeVidaRestante` (- (`self.TiempoDeVidaRestante`) DeltaSeconds)))
  (if (<= _output_get 0.0)
    ;[1 0.2705 0.7965] Le indica al GameManagerActor que ya acabó
    (bind _returnvalue (`GameplayStatics.GetActorOfClass` "/Game/Blueprints/GameManagerActor.GameManagerActor_C"))
    (`/Game/Blueprints/GameManagerActor.EndMiniGame` _returnvalue self)))

(fn `UserConstructionScript`)