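; MaterialChanger is a utility Blueprint that swaps the material on an array of static mesh actors across server and clients.
; RunOnServer takes an index into the Materials array and calls CambiarMaterial for each mesh, which is commented as a multicast and sets material slot 0.
; A test timer started on BeginPlay calls RunOnServer with the first material after a short delay.
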(event `RunOnServer`
  (params (Indice :type Integer))
  ;[1 1 1] CorreEventENServer
  (for _array_element (`self.Mesh`)
    (`self.CambiarMaterial` _array_element (`|GetArrayItem` (`self.materials`) Indice))))

(event `self.ReceiveBeginPlay`
  ;[0.2708 0.1707 0.1041] Test
  (`KismetSystemLibrary.K2_SetTimer` null "Test" 1.0))

(event `CambiarMaterial`
  (params (mesh :type "StaticMeshActor Object Reference") (material :type "Material Object Reference"))
  ;[0.4163 1 0.9801] Este evento usa multicast
  ; para reproducir en server y clientes
  (`PrimitiveComponent.SetMaterial` (`StaticMeshActor.StaticMeshComponent` mesh) 0 material))

(fn `Test`
  (`self.RunOnServer` 0))

(fn `UserConstructionScript`)