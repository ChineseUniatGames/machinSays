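; A toggleable platform for a "floor is lava" section that moves between its placed position and a point at the same X and Y with world Z zero.
; Activar flips the active state, and Tick, on authority only, moves a clamped alpha toward one or zero at a set speed.
; That alpha lerps the actor location without sweep.
; Resetear deactivates the platform and snaps it back to its starting position.
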(event `self.ReceiveBeginPlay`
  (bind _output_get (set `self.AlturaBaja` (`self.K2_GetActorLocation`)))
  (set `self.AlturaAlta` (`KismetMathLibrary.MakeVector` (.x _output_get) (.y _output_get))))

(event `/Game/Blueprints/Interfaces/IActivable.Activar`
  (params (Tiempo :type "Float (single-precision)"))
  (set `self.Activo` (not (`self.Activo`))))

(event `self.ReceiveTick`
  (params (DeltaSeconds :type "Float (single-precision)"))
  (bind _alfa (`self.Alfa`))
  (bind _alfa_2 (`self.Alfa`))
  (bind _returnvalue (* DeltaSeconds (`self.Speed`)))
  (`/Engine/EditorBlueprintResources/ActorMacros.Switch Has Authority`
    (:`Authority`
      (if (`self.Activo`)
        (if (< _alfa_2 1.0)
          (set `self.Alfa` (`KismetMathLibrary.FClamp` (+ _alfa_2 _returnvalue)))
          (`self.K2_SetActorLocation` (`KismetMathLibrary.VLerp` (`self.AlturaBaja`) (`self.AlturaAlta`) (`self.Alfa`)) :!label _label))
        (elif (> _alfa 0.0)
          (set `self.Alfa` (`KismetMathLibrary.FClamp` (- _alfa _returnvalue)))
          (goto _label))))))

(event `/Game/Blueprints/Interfaces/IReseteable.Resetear`
  ;[1 0.3528 0.9657] Reseteo
  (set `self.Activo` false)
  (set `self.Alfa` 0.0)
  (`self.K2_SetActorLocation` (`self.AlturaBaja`)))

(fn `UserConstructionScript`)