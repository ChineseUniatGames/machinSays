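; ObjetoLadoALado is a moving hazard actor that travels along world X and damages players it hits.
; On authority, Tick offsets it by Velocidad without sweep, not steering toward Objetivo, and destroys it within 10 units of that point.
; Mesh hits on Player-tagged actors apply Danio, also only on authority, then destroy it.
; Destruction chains through DestruirmeEnServer to DestruirmeEnMulti, named as server and multicast events.
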(event `self.ReceiveTick`
  (params (DeltaSeconds :type "Float (single-precision)"))
  (`/Engine/EditorBlueprintResources/ActorMacros.Switch Has Authority`
    (:`Authority`
      (if (<= (`KismetMathLibrary.Vector_Distance` (`self.Objetivo`) (`self.K2_GetActorLocation`)) 10.0)
        (`self.DestruirmeEnServer`)
        (else
          (`self.K2_AddActorWorldOffset` (`KismetMathLibrary.MakeVector` (* DeltaSeconds (`self.Velocidad`)))))))))

(event `self.StaticMesh.OnComponentHit`
  (params (HitComponent :type "PrimitiveComponent Object Reference") (OtherActor :type "Actor Object Reference") (OtherComp :type "PrimitiveComponent Object Reference") (NormalImpulse :type "Vector Structure") (Hit :type "HitResult Structure (by ref)"))
  (`/Engine/EditorBlueprintResources/ActorMacros.Switch Has Authority`
    (:`Authority`
      (if (`self.ActorHasTag` OtherActor "Player")
        (`GameplayStatics.ApplyDamage` OtherActor (`self.Danio`))
        (`self.DestruirmeEnServer`)))))

(event `DestruirmeEnServer`
  (`self.DestruirmeEnMulti`))

(event `DestruirmeEnMulti`
  (`self.K2_DestroyActor`))

(fn `UserConstructionScript`)