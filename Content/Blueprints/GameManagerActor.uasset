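; GameManagerActor runs the minigame loop, spawning a random minigame on BeginPlay.
; NewMiniGame picks a random index from ListaMiniJuegos, spawns that class at the origin and sends it an Activar message with its configured duration.
; EndMiniGame destroys the given minigame manager and immediately starts another random one.
; The JugadorMuerto event only prints a death message and the name of its parameter.
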(event `JugadorMuerto`
  (params (NewParam :type "Actor Object Reference"))
  ;[1 0.06134 0.04144] Jugador Muerto
  (`KismetSystemLibrary.PrintString` "Un compa murió")
  (`KismetSystemLibrary.PrintString` (`KismetSystemLibrary.GetDisplayName` NewParam)))

(event `self.ReceiveBeginPlay`
  ;[0 0.8813 1] Start mini games
  (`KismetSystemLibrary.PrintString` "Hello there")
  (`self.NewMiniGame`))

(fn `EndMiniGame`
  (params (MiniManager :type "Actor Object Reference"))
  (`KismetSystemLibrary.PrintString` "End mini game")
  (`self.K2_DestroyActor` MiniManager)
  (`self.NewMiniGame`))

(fn `NewMiniGame`
  (bind (_minijuego _tiempoporminijuego) (break `/Game/Blueprints/SMiniJuegos` (`self.ListaMiniJuegos`)))
  (bind _output_get (set `self.IndexActual` (`KismetMathLibrary.RandomIntegerInRange` 0 (- (`KismetArrayLibrary.Array_Length` _minijuego) 1))))
  (bind _returnvalue (`|SpawnActorFromClass` (`|GetArrayItem` _minijuego _output_get) (`KismetMathLibrary.MakeTransform` (0.0 0.0 0.0)) "Undefined" "OverrideRootScale" null null))
  (message `/Game/Blueprints/Interfaces/IActibable.Activar` _returnvalue (`|GetArrayItem` _tiempoporminijuego _output_get)))

(fn `UserConstructionScript`)