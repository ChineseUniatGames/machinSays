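; SafeZone is an actor that marks a safe area which can be activated and deactivated during play.
; Activar calls setInserver, which moves the zone to a random XY spot within a fixed square just above the origin plane.
; Desactivar hides it by moving it below the ground at the origin.
; Overlap begin and end on the Zonitasegura component set or clear EnSafeZone on any ThirdPersonCharacter.
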(event `/Game/Blueprints/Interfaces/IActivable.Activar`
  (params (Tiempo :type "Float (single-precision)"))
  (`self.setInserver`))

(event `setInserver`
  (`self.K2_SetActorLocation` (`KismetMathLibrary.MakeVector` (`KismetMathLibrary.RandomFloatInRange` -1000.0 1000.0) (`KismetMathLibrary.RandomFloatInRange` -1000.0 1000.0) 10.0)))

(event `desactivar`
  (`self.K2_SetActorLocation` (0.0 0.0 -50.0)))

(event `self.zonitasegura.OnComponentBeginOverlap`
  (params (OverlappedComponent :type "PrimitiveComponent Object Reference") (OtherActor :type "Actor Object Reference") (OtherComp :type "PrimitiveComponent Object Reference") (OtherBodyIndex :type Integer) (bFromSweep :type Boolean) (SweepResult :type "HitResult Structure (by ref)"))
  (bind _asthird_person_character (cast `/Game/ThirdPersonBP/Blueprints/ThirdPersonCharacter` OtherActor))
  (set `/Game/ThirdPersonBP/Blueprints/ThirdPersonCharacter.enSafeZone` true _asthird_person_character))

(event `self.zonitasegura.OnComponentEndOverlap`
  (params (OverlappedComponent :type "PrimitiveComponent Object Reference") (OtherActor :type "Actor Object Reference") (OtherComp :type "PrimitiveComponent Object Reference") (OtherBodyIndex :type Integer))
  (bind _asthird_person_character (cast `/Game/ThirdPersonBP/Blueprints/ThirdPersonCharacter` OtherActor))
  (set `/Game/ThirdPersonBP/Blueprints/ThirdPersonCharacter.enSafeZone` false _asthird_person_character))

(fn `UserConstructionScript`)