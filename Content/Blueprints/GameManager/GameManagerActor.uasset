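; Game manager actor that runs a sequence of mini-games and handles player death and resets.
; NewMiniGame spawns a random or forced entry from ListaMiniJuegos and activates it with its time; EndMiniGame destroys it and starts another.
; JugadorMuerto destroys the dead player through JugadorMuertoMulti.
; BtnReset messages IReseteable actors, recreates characters at "Spawn"-tagged actors, possesses them by controller index, then starts a new mini-game after a delay.
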(event `JugadorMuerto`
  (params (NewParam :type "Actor Object Reference"))
  ;[1 0.06134 0.04144] Jugador Muerto
  (`KismetSystemLibrary.PrintString` "Un compa murió")
  (`KismetSystemLibrary.PrintString` (`KismetSystemLibrary.GetDisplayName` NewParam))
  (`self.JugadorMuertoMulti` NewParam))

(event `self.ReceiveBeginPlay`
  ;[0 0.8813 1] Start mini games
  (`KismetSystemLibrary.PrintString` "Hello there")
  (`self.NewMiniGame`))

(event `JugadorMuertoMulti`
  (params (Player :type "Actor Object Reference"))
  ;[1 0.1521 0.2319] JugadorMuertoMulti
  (`self.K2_DestroyActor` Player))

(event `BtnReset`
  ;[1 0.902 0] Reseteo
  (bind _outactors (`GameplayStatics.GetAllActorsWithInterface` "/Game/Blueprints/Interfaces/IReseteable.IReseteable_C"))
  (for _array_element _outactors
    (message `/Game/Blueprints/Interfaces/IReseteable.Resetear` _array_element))
  (bind _outactors_2 (`GameplayStatics.GetAllActorsOfClass` "/Game/ThirdPersonBP/Blueprints/ThirdPersonCharacter.ThirdPersonCharacter_C"))
  (for _array_element_2 _outactors_2
    (`self.K2_DestroyActor` _array_element_2))
  (`self.ReinstancearJugadores`)
  (`KismetSystemLibrary.Delay` 3.0)
  (`KismetSystemLibrary.PrintString` "Reseteado" true true (struct :`R` 0.252667 :`G` 1.0 :`A` 1.0) 5.0)
  (`self.NewMiniGame`))

(event `ReinstancearJugadores`
  ;[0.1946 0.9303 1] Reinstanciar jugadores
  (bind _outactors (`GameplayStatics.GetAllActorsWithTag` "Spawn"))
  (for (_array_element _array_index) _outactors
    (bind _returnvalue (`|SpawnActorFromClass` "/Game/ThirdPersonBP/Blueprints/ThirdPersonCharacter.ThirdPersonCharacter_C" (`KismetMathLibrary.MakeTransform` (`self.K2_GetActorLocation` _array_element)) "Undefined" "OverrideRootScale" null null))
    (`Controller.Possess` (`GameplayStatics.GetPlayerController` _array_index) _returnvalue)
    (`/Game/ThirdPersonBP/Blueprints/ThirdPersonCharacter.Reposeer` _returnvalue)))

(fn `EndMiniGame`
  (params (MiniManager :type "Actor Object Reference"))
  (`KismetSystemLibrary.PrintString` "End mini game")
  (`self.K2_DestroyActor` MiniManager)
  (`self.NewMiniGame`))

(fn `NewMiniGame`
  (bind _returnvalue (`KismetMathLibrary.MakeTransform` (0.0 0.0 0.0)))
  (bind _forzarminigame (`self.ForzarMiniGame`))
  (bind (_minijuego _tiempoporminijuego) (break `/Game/Blueprints/SMiniJuegos` (`self.ListaMiniJuegos`)))
  (bind (_minijuego_2 _tiempoporminijuego_2) (break `/Game/Blueprints/SMiniJuegos` (`self.ListaMiniJuegos`)))
  (if (>= (`self.ForzarMiniGame`) 0)
    (bind _returnvalue_2 (`|SpawnActorFromClass` (`|GetArrayItem` _minijuego _forzarminigame) _returnvalue "Undefined" "OverrideRootScale" null null))
    (message `/Game/Blueprints/Interfaces/IActivable.Activar` _returnvalue_2 (`|GetArrayItem` _tiempoporminijuego _forzarminigame))
    (else
      (bind _output_get (set `self.IndexActual` (`KismetMathLibrary.RandomIntegerInRange` 0 (- (`KismetArrayLibrary.Array_Length` _minijuego_2) 1))))
      (bind _returnvalue_3 (`|SpawnActorFromClass` (`|GetArrayItem` _minijuego_2 _output_get) _returnvalue "Undefined" "OverrideRootScale" null null))
      (message `/Game/Blueprints/Interfaces/IActivable.Activar` _returnvalue_3 (`|GetArrayItem` _tiempoporminijuego_2 _output_get)))))

(fn `UserConstructionScript`)