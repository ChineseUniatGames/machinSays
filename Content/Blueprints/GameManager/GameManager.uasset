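; GameManager runs the game's loop of random mini-games, starting one on BeginPlay.
; NewMiniGame picks a random entry from ListMiniJuegos, spawns that mini-game actor at the origin and passes its time to ActivarMessage.
; EndMiniGame destroys the finished mini-game's manager and starts the next one.
; JugadorMuerto only prints player deaths, and the remaining-time countdown is left unconnected.
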(event `JugadorMuerto`
  (params (NewParam :type "Actor Object Reference"))
  ;[1 0.06134 0.04144] Jugador Muerto
  (`KismetSystemLibrary.PrintString` "Un compa murió")
  (`KismetSystemLibrary.PrintString` (`KismetSystemLibrary.GetDisplayName` NewParam)))

(event `self.ReceiveBeginPlay`
  ;[0 0.8813 1] Start mini games
  (`KismetSystemLibrary.PrintString` "Hello there")
  (`self.NewMiniGame`))

(event `self.ReceiveTick`
  (params (DeltaSeconds :type "Float (single-precision)")))

(fn `EndMiniGame`
  (params (MiniManager :type "Actor Object Reference"))
  (`KismetSystemLibrary.PrintString` "MiniJuego terminado")
  (`self.K2_DestroyActor` MiniManager)
  (`self.NewMiniGame`))

(fn `NewMiniGame`
  (bind (_minijuego _tiempoporminijuego) (break `/Game/Blueprints/SMiniJuegos` (`self.ListMiniJuegos`)))
  (bind _output_get (set `self.IndexActual` (`KismetMathLibrary.RandomIntegerInRange` 0 (- (`KismetArrayLibrary.Array_Length` _minijuego) 1))))
  (bind _returnvalue (`|SpawnActorFromClass` (`|GetArrayItem` _minijuego _output_get) (`KismetMathLibrary.MakeTransform` (0.0 0.0 0.0)) "Undefined" "OverrideRootScale" null null))
  (message `/Game/Blueprints/Interfaces/IActibable.Activar` _returnvalue (`|GetArrayItem` _tiempoporminijuego _output_get))
  (`KismetSystemLibrary.PrintString` "MiniJuego activado"))

(fn `UserConstructionScript`)