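; SkinManager runs the timed skin selection phase that precedes a minigame.
; On BeginPlay or Activar it spawns a grid of six SkinSelector actors, each given a mesh from StaticMeshes.
; After a short delay it calls ShowMoneditas on every ThirdPersonCharacter to show their widgets.
; A 16-second timer then destroys all selectors and calls NewMiniGame on the GameManagerActor.
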(event `putWidgetTOPlayers`
  ;[0.001142 0 1] ponerlesWidgets
  (`KismetSystemLibrary.Delay` 1.0)
  (bind _outactors (`GameplayStatics.GetAllActorsOfClass` "/Game/ThirdPersonBP/Blueprints/ThirdPersonCharacter.ThirdPersonCharacter_C"))
  (for _array_element _outactors
    (`KismetSystemLibrary.PrintString` "Poniendo Widgets" true true (struct :`R` 0.412548 :`B` 1.0 :`A` 1.0) 10.0)
    (`/Game/ThirdPersonBP/Blueprints/ThirdPersonCharacter.ShowMoneditas` _array_element)))

(event `self.ReceiveBeginPlay`
  ;[1 0.05658 0] Iniciar
  (`self.ponerSkins` :!label _label)
  (`KismetSystemLibrary.K2_SetTimer` null "destroyAndSpawn" 16.0)
  (`self.putWidgetTOPlayers`))

(event `/Game/Blueprints/Interfaces/IActivable.Activar`
  (params (Tiempo :type "Float (single-precision)"))
  ;[1 0.05658 0] Iniciar
  (goto _label))

(event `ponerSkins`
  (bind _meshindex (`self.meshIndex`))
  ;[0.6037 0.4074 1] KK
  (for _ (range 3)
    (for _ (range 2)
      (bind _returnvalue (`|SpawnActorFromClass` "/Game/Blueprints/SkinSelector.SkinSelector_C" (`KismetMathLibrary.MakeTransform` (`self.indexPose`) (struct :`Yaw` 90.0)) "Undefined" "OverrideRootScale" null null))
      (set `/Game/Blueprints/SkinSelector.meshVar` (`|GetArrayItem` (`self.staticMeshes`) _meshindex) _returnvalue)
      (`/Game/Blueprints/SkinSelector.actualizar` _returnvalue)
      (`/Engine/EditorBlueprintResources/StandardMacros.IncrementInt` _meshindex
        (:`  `
          (set `self.indexPose` (+ (`self.indexPose`) (800.0 0.0 0.0))))))
    (set `self.indexPose` (+ (`self.indexPose`) (-1600.0 800.0 0.0))))
  (set `self.indexPose` (`self.InitialPose`))
  (set `self.meshIndex` 0))

(event `ponerGAmeManager`
  ;[0.02566 1 0] ponergamemanager
  (bind _returnvalue (`GameplayStatics.GetActorOfClass` "/Game/Blueprints/GameManager/GameManagerActor.GameManagerActor_C"))
  (`/Game/Blueprints/GameManager/GameManagerActor.NewMiniGame` _returnvalue))

(fn `destroyAndSpawn`
  (bind _outactors (`GameplayStatics.GetAllActorsOfClass` "/Game/Blueprints/SkinSelector.SkinSelector_C"))
  (bind _output_get (set `self.skinsSelect` _outactors))
  (for _array_element _output_get
    (`self.K2_DestroyActor` _array_element))
  (`self.ponerGAmeManager`))

(fn `UserConstructionScript`)